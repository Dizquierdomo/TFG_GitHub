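; Player character Blueprint with a toggleable enemy lock-on that steers the camera.
; EnemyFocusRadius overlaps store the latest ENEMY-tagged actor as SelectedEnemy, and any such actor leaving clears selection and lock, with debug prints.
; The TargetEnemy input toggles the lock when an enemy is selected.
; While locked, Tick drives control pitch and yaw toward the enemy via RInterpTo, preserving roll, and enables CameraBoom lag.
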(event OnComponentBeginOverlap(EnemyFocusRadius)
  (params (OverlappedComponent :type Primitive%20Component%20Object%20Reference) (OtherActor :type Actor%20Object%20Reference) (OtherComp :type Primitive%20Component%20Object%20Reference) (OtherBodyIndex :type Integer) (bFromSweep :type Boolean) (SweepResult :type Hit%20Result%20Structure%20%28by%20ref%29))
  (if (Actor|ActorHasTag OtherActor "ENEMY")
    (bind _output_get (Variables|Default|SetSelectedEnemy OtherActor))
    (Development|PrintString (Utilities|String|ToString(Name) (Utilities|Array|Get(acopy) (Variables|/Script/Engine.Actor|GetTags _output_get))) true true "(R=0.090973,G=1.000000,B=0.026334,A=1.000000)")))

(event OnComponentEndOverlap(EnemyFocusRadius)
  (params (OverlappedComponent :type Primitive%20Component%20Object%20Reference) (OtherActor :type Actor%20Object%20Reference) (OtherComp :type Primitive%20Component%20Object%20Reference) (OtherBodyIndex :type Integer))
  (if (Actor|ActorHasTag OtherActor "ENEMY")
    (Variables|Default|SetSelectedEnemy 0)
    (Development|PrintString (Utilities|String|ToString(Name) (Utilities|Array|Get(acopy) (Variables|/Script/Engine.Actor|GetTags OtherActor))) true true "(R=1.000000,G=0.045011,B=0.000000,A=1.000000)")
    (Variables|Default|SetIsEnemyTargeted false)))

(event EventTick
  (params (DeltaSeconds :type Float%20%28single-precision%29))
  (bind _returnvalue (Pawn|GetController))
  (bind _returnvalue_2 (Transformation|GetActorLocation))
  (bind _returnvalue_3 (Utilities|Time|GetWorldDeltaSeconds))
  (bind _selectedenemy (Variables|Default|GetSelectedEnemy))
  (bind _cameraboom (Variables|Default|GetCameraBoom))
  (bind _cameraboom_2 (Variables|Default|GetCameraBoom))
  (bind _returnvalue_4 (Pawn|GetControlRotation _returnvalue :!class /Script/Engine.Controller))
  (bind _returnvalue_5 (Transformation|GetActorLocation _selectedenemy))
  (bind _returnvalue_6 (Math|Rotator|FindLookatRotation _returnvalue_2 _returnvalue_5))
  (bind _returnvalue_7 (Math|Interpolation|RInterpTo _returnvalue_4 _returnvalue_6 _returnvalue_3 0.0))
  (if (Variables|Default|GetIsEnemyTargeted)
    (Pawn|SetControlRotation _returnvalue (Math|Rotator|MakeRotator (.Roll (Math|Rotator|BreakRotator _returnvalue_4)) (.pitch _returnvalue_7) (.yaw _returnvalue_7)))
    (Variables|/Script/Engine.SpringArmComponent|SetbEnableCameraLag _cameraboom_2 true)
    (Variables|/Script/Engine.SpringArmComponent|SetCameraLagSpeed _cameraboom_2 3.0)
    (else
      (Variables|/Script/Engine.SpringArmComponent|SetbEnableCameraLag _cameraboom false)
      (Variables|/Script/Engine.SpringArmComponent|SetCameraLagSpeed _cameraboom 0.0))))

(event Input|ActionEvents|InputActionTargetEnemy
  (params (Key :type Key%20Structure :default "None"))
  (:Pressed
    (if (Variables|Default|GetIsEnemyTargeted)
      (Variables|Default|SetIsEnemyTargeted false)
      (else
        (Utilities|Casting|CastToActor (Variables|Default|GetSelectedEnemy)
          (:then
            (Variables|Default|SetIsEnemyTargeted true))
          (:CastFailed
            (Development|PrintString "CAST FAIL !!!!" true true "(R=1.000000,G=0.045011,B=0.000000,A=1.000000)")))))))

(fn ConstructionScript)